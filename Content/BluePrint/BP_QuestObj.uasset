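; BP_QuestObj is a quest object that tracks a list of collectible-based objectives and its own started and finished state.
; UpdateObjectif adds a collectible's value to the first objective of matching type, then CheckObjectif marks it finished once it reaches its maximum.
; When every objective is finished, CheckQuestObjectif finishes the quest and calls MissionComplete on the GameInstance's current widget.
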(fn CheckQuestObjectif
  (for _array_element (Variables|Default|GetObjectifs)
    (if (not (.IsFinished (Utilities|Struct|BreakST_Objectif _array_element)))
      (return)))
  (CallFunction|QuestFinish)
  (Default|MissionComplete (Variables|/Game/BluePrint/Game/BP_GameInstance.BP_GameInstance_C|GetCurrentWidget (Variables|Default|GetGameInstance))))

(fn UpdateObjectif
  (params (Collectible :type BP%20Collectible%20Object%20Reference))
  (bind _objectifs (Variables|Default|GetObjectifs))
  (bind _index (Utilities|FlowControl|ForLoopwithBreak 0 (- (Utilities|Array|Length _objectifs) 1))
    (:LoopBody
      (if (Utilities|Enum|Equal(Enum) (.CollectibleType (Utilities|Struct|BreakST_Objectif (Utilities|Array|Get(acopy) _objectifs _index))) (Variables|/Game/BluePrint/Collectible/BP_Collectible.BP_Collectible_C|GetCollectibleType Collectible))
        (Utilities|Struct|SetmembersinST_Objectif (Utilities|Array|Get(acopy) _objectifs _index) (+ (.ActuelValue (Utilities|Struct|BreakST_Objectif (Utilities|Array|Get(acopy) _objectifs _index))) (Variables|/Game/BluePrint/Collectible/BP_Collectible.BP_Collectible_C|GetValue Collectible)))
        (CallFunction|CheckObjectif _index)
        (return)))))

(fn CheckObjectif
  (params (NumObject :type Integer))
  (bind _objectifs (Variables|Default|GetObjectifs))
  (bind _output (Utilities|Array|Get(acopy) _objectifs NumObject))
  (bind (_name _maxvalue _actuelvalue) (Utilities|Struct|BreakST_Objectif _output))
  (if (>= _actuelvalue _maxvalue)
    (bind _structout (Utilities|Struct|SetmembersinST_Objectif _output true))
    (Utilities|Array|SetArrayElem (Variables|Default|GetObjectifs) NumObject _structout)
    (CallFunction|CheckQuestObjectif))
  (return))

(fn QuestFinish
  (Variables|Default|SetIsFinished true)
  (Variables|Default|SetIsStart false))

(fn QuestStart
  (Variables|Default|SetIsStart true)
  (Variables|Default|SetIsFinished false))