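; BP_Plate is a plate whose Cube automatically moves up and down on a repeating cycle.
; After a startup delay of WaitTime, a looping timer fires Move, which plays or reverses the Up timeline depending on IsUp.
; The timeline lerps the cube's height between its starting Z and UpDistance above it, then flips IsUp on finishing.
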(event Custom|Move
  (bind _location (Variables|Default|GetLocation))
  (if (Variables|Default|GetIsUp)
    (bind _uptrack (Timeline|Up Reverse)
      (:Update
        (Transformation|SetWorldLocation (Variables|Default|GetCube) (Math|Vector|MakeVector (.x _location) (.y _location) (Math|Float|Lerp (.z _location) (+ (.z _location) (Variables|Default|GetUpDistance)) _uptrack)) false false))
      (:Finished
        (if (Variables|Default|GetIsUp)
          (Variables|Default|SetIsUp false)
          (else
            (Variables|Default|SetIsUp true)))
        (Utilities|FlowControl|Delay 2.0)))
    (else
      (Timeline|Up PlayFromStart))))

(event EventBeginPlay
  (Variables|Default|SetLocation (Transformation|GetWorldLocation (Variables|Default|GetCube)))
  (Utilities|FlowControl|Delay (Variables|Default|GetWaitTime))
  (Utilities|Time|SetTimerbyEvent (delegate Custom|Move) 7.0 true))

(event Collision|EventActorBeginOverlap
  (params (OtherActor :type Actor%20Object%20Reference)))

(event EventTick
  (params (DeltaSeconds :type Float%20%28single-precision%29)))

(fn ConstructionScript)