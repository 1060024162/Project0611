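; BP_PlateRotate is an interactable plate actor whose Cube mesh flips over periodically.
; On BeginPlay it caches the cube's world rotation, waits a configurable WaitTime, then starts a looping five-second timer.
; Each timer tick plays the Up timeline from the start, lerping pitch 180 degrees from the cached starting rotation, so every flip begins from that same orientation.
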(event Custom|Rotate
  (bind _rotation (Variables|Default|GetRotation))
  (bind _uptrack (Timeline|Up PlayFromStart)
    (:Update
      (Transformation|SetWorldRotation (Variables|Default|GetCube) (Math|Rotator|MakeRotator (.roll _rotation) (Math|Float|Lerp (.pitch _rotation) (+ (.pitch _rotation) 1.8e+02) _uptrack) (.yaw _rotation)) false false))))

(event EventBeginPlay
  (Variables|Default|SetRotation (Transformation|GetWorldRotation (Variables|Default|GetCube)))
  (Utilities|FlowControl|Delay (Variables|Default|GetWaitTime))
  (Utilities|Time|SetTimerbyEvent (delegate Custom|Rotate) 5.0 true))

(event Collision|EventActorBeginOverlap
  (params (OtherActor :type Actor%20Object%20Reference)))

(event EventTick
  (params (DeltaSeconds :type Float%20%28single-precision%29)))

(fn ConstructionScript)